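; Spell component for BP_TopDownCharacter that runs speed and health regen buffs, one active spell at a time.
; Each spell reads its values from a data asset (DA_Spell_Speed, DA_Spell_Regen) into ActiveSpell.
; Speed raises walk speed above the cached base and starts a looping Duration timer whose handle is not stored.
; Regen heals on a one-second timer, clearing it and the spell at full HP or when duration expires.
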(event Custom|RegenTick
  (bind _asbp_top_down_character (Utilities|Casting|CastToBP_TopDownCharacter (Variables|Default|GetOwnerCharacter)))
  (if (> (Variables|Default|GetRemainingDuration) 0.0)
    (if (< (Variables|/Game/TopDown/Blueprints/BP_TopDownCharacter.BP_TopDownCharacter_C|GetCurrentHP _asbp_top_down_character) (Variables|/Game/TopDown/Blueprints/BP_TopDownCharacter.BP_TopDownCharacter_C|GetMaxHp _asbp_top_down_character))
      (bind _output_get (Variables|/Game/TopDown/Blueprints/BP_TopDownCharacter.BP_TopDownCharacter_C|SetCurrentHP _asbp_top_down_character (+ (Variables|/Game/TopDown/Blueprints/BP_TopDownCharacter.BP_TopDownCharacter_C|GetCurrentHP _asbp_top_down_character) (Variables|/Game/Blueprints/Data/BP_DA_Spell.BP_DA_Spell_C|GetHealthRegen (Variables|Default|GetActiveSpell)))))
      (if (> (Variables|/Game/TopDown/Blueprints/BP_TopDownCharacter.BP_TopDownCharacter_C|GetCurrentHP _asbp_top_down_character) (Variables|/Game/TopDown/Blueprints/BP_TopDownCharacter.BP_TopDownCharacter_C|GetMaxHp _asbp_top_down_character))
        (Variables|/Game/TopDown/Blueprints/BP_TopDownCharacter.BP_TopDownCharacter_C|SetCurrentHP _asbp_top_down_character (Variables|/Game/TopDown/Blueprints/BP_TopDownCharacter.BP_TopDownCharacter_C|GetMaxHp _asbp_top_down_character))
        (Utilities|Time|ClearandInvalidateTimerbyHandle (Variables|Default|GetRegenTimerHandle) :!label _label)
        (CallFunction|EndRegenSpell)
        (else
          (Variables|Default|SetRemainingDuration (- (Variables|Default|GetRemainingDuration) 1.0))
          (Development|PrintString (Utilities|String|ToString(Float) _output_get))
          (if (<= (Variables|Default|GetRemainingDuration) 0.0)
            (Development|PrintString "plus de dur")
            (goto _label)
            (else
              (Development|PrintString "1 Tick")))))
      (else
        (goto _label)))))

(event EventBeginPlay
  (bind _asbp_top_down_character (Utilities|Casting|CastToBP_TopDownCharacter (Components|GetOwner)))
  (bind _output_get (Variables|Default|SetOwnerCharacter _asbp_top_down_character))
  (Variables|Default|SetBaseWalkSpeed (Variables|/Script/Engine.CharacterMovementComponent|GetMaxWalkSpeed (Variables|/Script/Engine.Character|GetCharacterMovement _output_get))))

(fn ActivateSpeedSpell
  (if (!= (Variables|Default|GetActiveSpell) 0)
    (return)
    (else
      (Variables|Default|SetActiveSpell "/Game/Data/Spells/DA_Spell_Speed.DA_Spell_Speed")
      (Development|PrintText (Variables|/Game/Blueprints/Data/BP_DA_Spell.BP_DA_Spell_C|GetPopUpText (Variables|Default|GetActiveSpell)))
      (Variables|/Script/Engine.CharacterMovementComponent|SetMaxWalkSpeed (Variables|/Script/Engine.Character|GetCharacterMovement (Variables|Default|GetOwnerCharacter)) (+ (Variables|Default|GetBaseWalkSpeed) (Variables|/Game/Blueprints/Data/BP_DA_Spell.BP_DA_Spell_C|GetSpeedBonus (Variables|Default|GetActiveSpell))))
      (Utilities|Time|SetTimerbyEvent (EventDispatchers|CreateEvent :!event EndSpeedSpell) (Variables|/Game/Blueprints/Data/BP_DA_Spell.BP_DA_Spell_C|GetDuration (Variables|Default|GetActiveSpell)) true))))

(fn EndSpeedSpell
  (Variables|/Script/Engine.CharacterMovementComponent|SetMaxWalkSpeed (Variables|/Script/Engine.Character|GetCharacterMovement (Variables|Default|GetOwnerCharacter)) (Variables|Default|GetBaseWalkSpeed))
  (Variables|Default|SetActiveSpell 0)
  (Development|PrintString "fini"))

(fn ActivateRegenSpell
  (if (!= (Variables|Default|GetActiveSpell) 0)
    (return)
    (else
      (Variables|Default|SetActiveSpell "/Game/Data/Spells/DA_Spell_Regen.DA_Spell_Regen")
      (Variables|Default|SetRemainingDuration (Variables|/Game/Blueprints/Data/BP_DA_Spell.BP_DA_Spell_C|GetDuration (Variables|Default|GetActiveSpell)))
      (bind _returnvalue (Utilities|Time|SetTimerbyEvent (EventDispatchers|CreateEvent :!event Custom|RegenTick) 1.0 true))
      (Variables|Default|SetRegenTimerHandle _returnvalue)
      (Development|PrintString "aaaaa"))))

(fn EndRegenSpell
  (Variables|Default|SetActiveSpell 0)
  (Development|PrintString "Fin de regen"))