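; BP_Fireball is a fireball spell actor that damages top-down enemy characters on contact.
; Its sphere collision overlap passes SpellData's DamageBonus to the enemy's LooseHp, prints a debug message and destroys the fireball.
; Overlapping its owner also destroys it without damage, while other non-enemy actors fail the cast and leave it alive.
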(event OnComponentBeginOverlap(SphereCollision)
  (params (OverlappedComponent :type Primitive%20Component%20Object%20Reference) (OtherActor :type Actor%20Object%20Reference) (OtherComp :type Primitive%20Component%20Object%20Reference) (OtherBodyIndex :type Integer) (bFromSweep :type Boolean) (SweepResult :type Hit%20Result%20Structure%20%28by%20ref%29))
  (if (!= OtherActor (Components|GetOwner))
    (bind _asbp_top_down_character_enemy (Utilities|Casting|CastToBP_TopDownCharacterEnemy OtherActor))
    (Default|LooseHp _asbp_top_down_character_enemy (Variables|/Game/Blueprints/Data/BP_DA_Spell.BP_DA_Spell_C|GetDamageBonus (Variables|Default|GetSpellData)))
    (Development|PrintString "Touché")
    (Actor|DestroyActor)
    (else
      (Actor|DestroyActor))))

(fn ConstructionScript)